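; Tutorial map actor that applies a simple fake gravity to every Sil actor in the level.
; Each Tick it gathers all Sil actors and lowers any above a fixed world height by a constant step, without sweep or delta-time scaling, so fall speed follows frame rate.
; Overlap and BeginPlay events are empty, and a Hero tag check is left unconnected.
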(event EventBeginPlay)

(event Collision|EventActorBeginOverlap
  (params (OtherActor :type Actor%20Object%20Reference)))

(event EventTick
  (params (DeltaSeconds :type Float%20%28single-precision%29))
  (bind _outactors (Actor|GetAllActorsOfClass "/Game/Map_Tuto/Blueprint/Sil.Sil_C"))
  (for _array_element _outactors
    (if (> (.Z (Math|Vector|BreakVector (Transformation|GetActorLocation _array_element))) 2e+01)
      (Transformation|SetActorLocation _array_element (Math|Vector|MakeVector (.X (Math|Vector|BreakVector (Transformation|GetActorLocation _array_element))) (.Y (Math|Vector|BreakVector (Transformation|GetActorLocation _array_element))) (- (.Z (Math|Vector|BreakVector (Transformation|GetActorLocation _array_element))) 5.0)) false false))))

(fn ConstructionScript)